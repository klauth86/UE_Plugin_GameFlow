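; BP_Step_ShowHideWidget is a game flow step that shows a UI widget on enter and removes it on exit.
; On enter it synchronously loads the soft widget class, creates the widget for player controller 0 and adds it to the viewport.
; On exit it removes and clears the stored widget.
; Each event reports Finished only when its validity check passes, with no completion call otherwise.
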(event `self.OnEnter`
  (bind _userwidgetclass (`self.UserWidgetClass`))
  (if (`KismetSystemLibrary.IsValidSoftClassReference` _userwidgetclass)
    (bind _returnvalue (`KismetSystemLibrary.LoadClassAsset_Blocking` _userwidgetclass))
    (bind _asuser_widget (castclass `UserWidget` _returnvalue))
    (bind _returnvalue_2 (`|CreateWidget` _asuser_widget (`GameplayStatics.GetPlayerController` 0)))
    (bind _output_get (set `self.UserWidget` _returnvalue_2))
    (`UserWidget.AddToViewport` _output_get 0)
    (`self.OnComplete` "Finished")))

(event `self.OnExit`
  (bind _userwidget (`self.UserWidget`))
  (`/Engine/EditorBlueprintResources/StandardMacros.IsValid` _userwidget
    (:`Is Valid`
      (`Widget.RemoveFromParent` _userwidget)
      (set `self.UserWidget` null)
      (`self.OnComplete` "Finished"))))